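; BP_Player is the player pawn, which moves along world axes and turns to face the mouse cursor.
; Enhanced Input's IA_Move feeds movement input on fixed world X and negative Y, independent of facing, and BeginPlay shows the cursor.
; Each tick, a complex Visibility trace under the cursor supplies the look-at point, using only X and Y, and the actor rotates toward it at a constant TurnRate.
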(event Input|EnhancedActionEvents|EnhancedInputActionIA_Move
  (params (ActionValue :type Vector%202D%20Structure) (ElapsedSeconds :type Float%20%28double-precision%29) (TriggeredSeconds :type Float%20%28double-precision%29) (InputAction :type Input%20Action%20Object%20Reference :default "/Game/Input/Actions/IA_Move.IA_Move"))
  (:Triggered
    (Pawn|Input|AddMovementInput "1.000000,0.000000,0.000000" (.x ActionValue) false)
    (Pawn|Input|AddMovementInput "0.000000,-1.000000,0.000000" (.y ActionValue) false)))

(event EventBeginPlay
  (Variables|/Script/Engine.PlayerController|SetbShowMouseCursor (Game|GetPlayerController 0) true))

(event EventTick
  (params (DeltaSeconds :type Float%20%28single-precision%29))
  (|UpdatePlayerRotation DeltaSeconds))

(fn ConstructionScript)

(fn GetHitResultUnderCursorLocation
  (return (.location (.HitResult (Game|Player|GetHitResultUnderCursorbyChannel (Game|GetPlayerController 0) "TraceTypeQuery1" true)))))