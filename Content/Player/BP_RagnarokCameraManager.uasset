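; BP_RagnarokCameraManager adjusts the player camera's field of view according to how fast the controlled pawn moves.
; Every Tick, UpdateFOV finds the CameraComponent on player 0's pawn and compares the pawn's velocity length to a fixed threshold.
; SetFieldOfViewSmooth then uses FInterpTo to ease the FOV toward TargetFOV above that speed, or back to DefaultFOV otherwise.
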(event EventBeginPlay)

(event Collision|EventActorBeginOverlap
  (params (OtherActor :type Actor%20Object%20Reference)))

(event EventTick
  (params (DeltaSeconds :type Float%20%28single-precision%29))
  (|UpdateFOV DeltaSeconds))

(fn ConstructionScript)

(fn SetFieldOfViewSmooth
  (params (CurrentFieldOfView :type Float%20%28double-precision%29) (TargetFieldOfView :type Float%20%28double-precision%29) (DeltaTime :type Float%20%28double-precision%29) (InterpSpeed :type Float%20%28double-precision%29))
  (Camera|SetFieldOfView (Variables|Default|GetCameraComponent) (Math|Interpolation|FInterpTo CurrentFieldOfView TargetFieldOfView DeltaTime InterpSpeed)))