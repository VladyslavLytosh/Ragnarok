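; Base game mode that decides win and loss by tracking enemy and player deaths and showing the matching HUD screen.
; On BeginPlay it counts all BP_PunkAI actors and binds to their DeathComponent death-finished events; the player's binding sits inside the same loop, so it repeats per enemy.
; Punk deaths decrement the count, showing victory at zero if the player controls a valid pawn; player death shows the death screen.
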(event Custom|OnPlayerDeathFinished
  (bind _asbp_hud (Utilities|Casting|CastToBP_HUD (HUD|GetHUD (Game|GetPlayerController 0))))
  (Default|ShowDeathScreen _asbp_hud))

(event Custom|OnPunkDeathFinished
  (bind _returnvalue (Game|GetPlayerController 0))
  (bind _enemycount (Variables|Default|GetEnemyCount))
  (Math|Integer|DecrementInt _enemycount
    (:%20%20
      (if (and (<= _enemycount 0) (Utilities|IsValid (Pawn|GetControlledPawn _returnvalue)))
        (bind _asbp_hud (Utilities|Casting|CastToBP_HUD (HUD|GetHUD _returnvalue)))
        (Default|ShowVictoryScreen _asbp_hud)))))

(event EventBeginPlay
  (bind _outactors (Actor|GetAllActorsOfClass "/Game/AI/BP_PunkAI.BP_PunkAI_C"))
  (Variables|Default|SetEnemyCount (Utilities|Array|Length _outactors))
  (for _array_element _outactors
    (EventDispatchers|AssignOnCharacterDeathFinished (Variables|/Script/Ragrarok.BaseCharacter|GetDeathComponent _array_element) (delegate Custom|OnPunkDeathFinished))
    (bind _asbase_character (Utilities|Casting|CastToBaseCharacter (Game|GetPlayerCharacter 0)))
    (EventDispatchers|AssignOnCharacterDeathFinished (Variables|/Script/Ragrarok.BaseCharacter|GetDeathComponent _asbase_character) (delegate Custom|OnPlayerDeathFinished))))

(fn ConstructionScript)