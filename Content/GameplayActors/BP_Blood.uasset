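; Blood splat actor that drops a decal on the surface beneath it and plays a sound when spawned.
; BeginPlay traces downward and, on a hit, spawns a normal-aligned decal with a dynamic material, sized through GetRandomSize.
; A timeline at random play rate drives a scalar material parameter to animate the decal, then destroys the actor.
; Without a hit, nothing spawns and the actor is not destroyed here.
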(event EventBeginPlay
  ;[1 1 1] FATALNIY COD
  (bind (_outhit _returnvalue) (Class|KismetSystemLibrary|LineTraceSinglebyProfile (Transformation|GetActorLocation) (+ (Transformation|GetActorLocation) "0.000000,0.000000,-500.000000") "BlockAll" false 0 "None" true))
  (if _returnvalue
    (bind _returnvalue_2 (Rendering|Material|CreateDynamicMaterialInstance (Variables|Default|GetDecalMaterial) "None" "None" :!class /Script/Engine.KismetMaterialLibrary))
    (Rendering|Decal|SpawnDecalatLocation _returnvalue_2 (Utilities|GetRandomSize 5e+01 7e+01) (Math|Vector|MakeVector (.X (Class|KismetMathLibrary|BreakVector3f (.Location (Collision|BreakHitResult _outhit)))) (.Y (Class|KismetMathLibrary|BreakVector3f (.Location (Collision|BreakHitResult _outhit)))) (- (.Z (Class|KismetMathLibrary|BreakVector3f (.Location (Collision|BreakHitResult _outhit)))) (Variables|Default|GetZDecalOffset))) (Math|Rotator|MakeRotfromX (.Normal (Collision|BreakHitResult _outhit))) 0.0)
    (Components|Timeline|SetPlayRate (Variables|Default|GetTimeline) (Math|Random|RandomFloatinRange 0.5 1.0))
    (Audio|PlaySoundatLocation (Variables|Default|GetSound) (Transformation|GetActorLocation) "0, 0, 0" 1.0 1.0 0.0 0 0 0 0)
    (bind _time (Timeline|Timeline Play)
      (:Update
        (Rendering|Material|SetScalarParameterValue _returnvalue_2 (Variables|Default|GetMaterialParamName) _time :!class /Script/Engine.MaterialInstanceDynamic))
      (:Finished
        (Actor|DestroyActor)))))

(fn ConstructionScript)