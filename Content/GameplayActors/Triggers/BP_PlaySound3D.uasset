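; BP_PlaySound3D is a trigger actor that plays a configurable sound at its own location.
; If PlayAtBeginPlay is set the sound plays on BeginPlay, otherwise the first overlap of its Box component plays it once, with no filter on the overlapping actor.
; Both paths call PlaySound, a fire-and-forget PlaySoundAtLocation using the actor's volume, start time and attenuation variables.
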(event OnComponentBeginOverlap(Box)
  (params (OverlappedComponent :type Primitive%20Component%20Object%20Reference) (OtherActor :type Actor%20Object%20Reference) (OtherComp :type Primitive%20Component%20Object%20Reference) (OtherBodyIndex :type Integer) (bFromSweep :type Boolean) (SweepResult :type Hit%20Result%20Structure%20%28by%20ref%29))
  (if (not (Variables|Default|GetPlayAtBeginPlay))
    (Utilities|FlowControl|DoOnce false
      (:Completed
        (CallFunction|PlaySound)))))

(event EventBeginPlay
  (if (Variables|Default|GetPlayAtBeginPlay)
    (CallFunction|PlaySound)))

(event Collision|EventActorBeginOverlap
  (params (OtherActor :type Actor%20Object%20Reference)))

(event EventTick
  (params (DeltaSeconds :type Float%20%28single-precision%29)))

(fn ConstructionScript
  (|CallParentFunction))

(fn PlaySound
  (Audio|PlaySoundatLocation (Variables|Default|GetSound) (Transformation|GetActorLocation) (Transformation|GetActorRotation) (Variables|Default|GetVolume%20Multiplier) 1.0 (Variables|Default|GetStart%20Time) (Variables|Default|GetAttenuation%20Settings) 0 0 0))