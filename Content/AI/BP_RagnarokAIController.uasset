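; AI controller that runs a default behavior tree and feeds perception results into its Blackboard.
; When perception is enabled, each stimulus passes to sight, hearing and touch handlers, which filter by sense class.
; Sight and touch set or clear the player as target; lost sight stores the last location, while hearing stores a target location.
; Prediction handling exists but is disconnected, as is the prediction request.
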(event OnTargetPerceptionUpdated(AIPerception)
  (params (Actor :type Actor%20Object%20Reference) (Stimulus :type AI%20Stimulus%20Structure))
  (if (Variables|Default|GetEnableAIPerception)
    (CallFunction|HandleSightSense Actor Stimulus)
    (CallFunction|HandleSoundSense Stimulus)
    (CallFunction|HandleTouchEvent Stimulus Actor)))

(event EventBeginPlay
  (AI|RunBehaviorTree (Variables|Default|GetDefaultBTAsset)))

(fn ConstructionScript)

(fn HandleSightSense
  (params (Actor :type Actor%20Object%20Reference) (Stimulus :type AI%20Stimulus%20Structure))
  (bind _returnvalue (Class|AIPerceptionSystem|GetSenseClassforStimulus Stimulus))
  (if (== _returnvalue "/Script/AIModule.AISense_Sight")
    (if (== (CallFunction|GetPlayerCharacter) Actor)
      (AI|Components|Blackboard|SetValueasObject (Variables|Default|GetBlackboard) (Variables|Default|GetTarget%20Key%20Name) (Utilities|SelectObject (CallFunction|GetPlayerCharacter) 0 (.bsuccessfullysensed Stimulus)))
      (if (not (.bsuccessfullysensed Stimulus))
        (AI|Components|Blackboard|SetValueasVector (Variables|Default|GetBlackboard) (Variables|Default|GetLast%20Location%20Key%20Name) (.stimuluslocation Stimulus))))))

(fn GetPlayerCharacter
  (return (Game|GetPlayerCharacter 0)))

(fn HandleSoundSense
  (params (Stimulus :type AI%20Stimulus%20Structure%20%28by%20ref%29))
  (bind _returnvalue (Class|AIPerceptionSystem|GetSenseClassforStimulus Stimulus))
  (if (== _returnvalue "/Script/AIModule.AISense_Hearing")
    (AI|Components|Blackboard|SetValueasVector (Variables|Default|GetBlackboard) (Variables|Default|GetTarget%20Location%20Key%20Name) (.stimuluslocation Stimulus))))

(fn HandleTouchEvent
  (params (Stimulus :type AI%20Stimulus%20Structure%20%28by%20ref%29) (Actor :type Actor%20Object%20Reference))
  (bind _returnvalue (Class|AIPerceptionSystem|GetSenseClassforStimulus Stimulus))
  (if (== _returnvalue "/Script/AIModule.AISense_Touch")
    (if (== (CallFunction|GetPlayerCharacter) Actor)
      (AI|Components|Blackboard|SetValueasObject (Variables|Default|GetBlackboard) (Variables|Default|GetTarget%20Key%20Name) (Utilities|SelectObject (CallFunction|GetPlayerCharacter) 0 (.bsuccessfullysensed Stimulus))))))

(fn HandlePrediction
  (params (Stimulus :type AI%20Stimulus%20Structure%20%28by%20ref%29))
  (bind _returnvalue (Class|AIPerceptionSystem|GetSenseClassforStimulus Stimulus))
  (if (== _returnvalue "/Script/AIModule.AISense_Prediction")
    (AI|Components|Blackboard|SetValueasVector (Variables|Default|GetBlackboard) (Variables|Default|GetLast%20Location%20Key%20Name) (.stimuluslocation Stimulus))))