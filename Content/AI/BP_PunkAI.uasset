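; BP_PunkAI is a punk AI character that configures its character class and behavior when play begins.
; SetAIClass constructs DefaultPunkClass, assigns it to the CharacterClassComponent, then has the RagnarokAIController run the behavior tree mapped to that class in AIInfoMap, stored in a field named Blackboard.
; Missing class, controller or map entry prints an error.
; Actor overlaps are reported as touch events; a hardcoded BT_PunkWithKnife call is left unconnected.
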(event EventBeginPlay
  (CallFunction|SetAIClass))

(event Collision|EventActorBeginOverlap
  (params (OtherActor :type Actor%20Object%20Reference))
  (Class|AISenseTouch|ReportTouchEvent self OtherActor (Transformation|GetActorLocation)))

(fn ConstructionScript)

(fn SetAIClass
  (bind _aiinfomap (Variables|Default|GetAIInfoMap))
  (bind _defaultpunkclass (Variables|Default|GetDefaultPunkClass))
  (bind (_value _returnvalue) (Utilities|Map|Find _aiinfomap _defaultpunkclass))
  (if (Utilities|IsValidClass (Variables|Default|GetDefaultPunkClass))
    (bind _returnvalue_2 (Game|ConstructObjectfromClass (Variables|Default|GetDefaultPunkClass)))
    (Class|CharacterClassComponent|SetCurrentCharacterClass (Variables|Default|GetCharacterClassComponent) _returnvalue_2 self)
    (bind _asragnarok_aicontroller (Utilities|Casting|CastToRagnarokAIController (Pawn|GetController))
      (:then
        (if _returnvalue
          (AI|RunBehaviorTree _asragnarok_aicontroller (Utilities|Struct|BreakBP_AIClassInfo _value))
          (else
            (Development|PrintString "AI Class does not have ai class info" true true "(R=1.000000,G=0.202056,B=0.034016,A=1.000000)" 3.0))))
      (:CastFailed
        (Development|PrintString "AI Controller is not valid" true true "(R=1.000000,G=0.202056,B=0.034016,A=1.000000)" 3.0)))
    (else
      (Development|PrintString "AI Character class must be set" true true "(R=1.000000,G=0.202056,B=0.034016,A=1.000000)" 3.0))))